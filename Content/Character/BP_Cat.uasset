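; BP_Cat is a playable cat character with side-scroller style movement and collection of orbs as "peace fragments".
; BeginPlay registers the Enhanced Input mapping context, whose actions drive jumping, yaw look and movement along world X.
; Movement snaps control rotation to face forward or backward from the sign of X acceleration.
; The ObtenerOrbes event adds to the orb count and prints the collection message on screen.
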(event `self.ReceiveBeginPlay`
  (bind _asplayer_controller (cast `PlayerController` (`self.GetController`)))
  (`EnhancedInputSubsystemInterface.AddMappingContext` (pcsubsystem `EnhancedInputLocalPlayerSubsystem` _asplayer_controller) "/Game/Inputs/MapingContext/IMC_PersonajeInput.IMC_PersonajeInput" 0 (struct))
  (`KismetSystemLibrary.PrintString` "Mundo actual: \nAlta Gracia"))

(event `EnhancedInput|/Game/Inputs/InputActions/IA_Mirar`
  (params (ActionValue :type "Float (double-precision)") (ElapsedSeconds :type "Float (double-precision)") (TriggeredSeconds :type "Float (double-precision)") (InputAction :type "InputAction Object Reference" :default "/Game/Inputs/InputActions/IA_Mirar.IA_Mirar"))
  (:`Triggered`
    (`self.AddControllerYawInput` ActionValue)))

(event `EnhancedInput|/Game/Inputs/InputActions/IA_Movimiento`
  (params (ActionValue :type "Float (double-precision)") (ElapsedSeconds :type "Float (double-precision)") (TriggeredSeconds :type "Float (double-precision)") (InputAction :type "InputAction Object Reference" :default "/Game/Inputs/InputActions/IA_Movimiento.IA_Movimiento"))
  (bind _returnvalue (`self.GetController`))
  (bind _returnvalue_x (`KismetMathLibrary.BreakVector` (`CharacterMovementComponent.GetCurrentAcceleration` (`self.CharacterMovement`))))
  (:`Triggered`
    (`self.AddMovementInput` (1.0 0.0 0.0) ActionValue)
    (`/Engine/EditorBlueprintResources/StandardMacros.CompareFloat` _returnvalue_x
      (:`>`
        (`Controller.SetControlRotation` _returnvalue (`KismetMathLibrary.MakeRotator` 0.0)))
      (:`<`
        (`Controller.SetControlRotation` _returnvalue (`KismetMathLibrary.MakeRotator` 0.0 0.0 180.0))))))

(event `EnhancedInput|/Game/Inputs/InputActions/IA_Saltar`
  (params (ActionValue :type "Float (double-precision)") (ElapsedSeconds :type "Float (double-precision)") (TriggeredSeconds :type "Float (double-precision)") (InputAction :type "InputAction Object Reference" :default "/Game/Inputs/InputActions/IA_Saltar.IA_Saltar"))
  (:`Started`
    (`self.Jump`)))

(event `/Game/Interfaces/BPI_Recolectar.ObtenerOrbes`
  (params (Orbes :type Integer))
  (bind _output_get (set `self.Orbes` (+ Orbes (`self.Orbes`))))
  (`KismetSystemLibrary.PrintString` (`KismetStringLibrary.Concat_StrStr` "Recolectaste un fragmento de paz!  \nTus fragementos actuales son: " (`KismetStringLibrary.Conv_IntToString` _output_get)) true true (struct :`G` 0.66 :`B` 1.0 :`A` 1.0) 5.0))

(fn `UserConstructionScript`)